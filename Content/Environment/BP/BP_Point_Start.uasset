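; Start point actor that spawns an AI character and hands it its route.
; PressButton spawns the configured character at the Spawn component, applies the chosen skeletal mesh, then messages its AI controller with start and end points, timings and go/stop conditions.
; Separately, any overlap with the Box spawns a short-lived rotating shield actor at the FX transform and plays a 2D spawn sound.
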(event OnComponentBeginOverlap(Box)
  (params (OverlappedComponent :type Primitive%20Component%20Object%20Reference) (OtherActor :type Actor%20Object%20Reference) (OtherComp :type Primitive%20Component%20Object%20Reference) (OtherBodyIndex :type Integer) (bFromSweep :type Boolean) (SweepResult :type Hit%20Result%20Structure%20%28by%20ref%29))
  (bind _returnvalue (Game|SpawnActorfromClass "/Game/VFX/Blueprints/BP_Rotating_Shield.BP_Rotating_Shield_C" (Transformation|GetWorldTransform (Variables|Default|GetFX)) "AlwaysSpawn" 0 0))
  (Audio|PlaySound2D "/Game/Sounds/Sound_Spawn.Sound_Spawn" 1.0 1.0 0.0 0 0)
  (Utilities|FlowControl|Delay 1.5)
  (Actor|DestroyActor _returnvalue))

(event Custom|Press%20Button
  (bind _spawn (Variables|Default|GetSpawn))
  (bind _returnvalue (AI|SpawnAIFromClass (Variables|Default|GetBP_Character) 0 (Transformation|GetWorldLocation _spawn) (Transformation|GetWorldRotation _spawn) true 0))
  (Variables|Default|SetSet%20Character _returnvalue)
  (Class|SkinnedMeshComponent|SetSkeletalMesh (Actor|GetComponentbyClass _returnvalue "/Script/Engine.SkeletalMeshComponent") (Variables|Default|GetSkeletalMash) true)
  (Class|BIAIController|SendAIController(Message) (AI|GetAIController (Variables|Default|GetSet%20Character)) (Variables|SpawnChar|GetStartPoint) (Variables|SpawnChar|GetEndPoint) (Variables|SpawnChar|GetTimeToEnd) (Variables|SpawnChar|GetTimeToStart) (Variables|SpawnChar|GetCondition%20Go) (Variables|SpawnChar|GetCondition%20Stop) (Variables|SpawnChar|GetStopTime)))

(event EventBeginPlay
  (|CallParentFunction))

(event Collision|EventActorBeginOverlap
  (params (OtherActor :type Actor%20Object%20Reference))
  (|CallParentFunction OtherActor) ; This node is disabled and will not be called.\nDrag off pins to build functionality.
)

(event EventTick
  (params (DeltaSeconds :type Float%20%28single-precision%29))
  (|CallParentFunction DeltaSeconds) ; This node is disabled and will not be called.\nDrag off pins to build functionality.
)

(fn ConstructionScript
  (|CallParentFunction))